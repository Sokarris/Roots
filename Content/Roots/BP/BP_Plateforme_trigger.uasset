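; BP_Plateforme_trigger is a moving platform that travels along a spline when the third-person character enters its trigger.
; A FlipFlop on overlap alternates between playing and reversing the PlateformMovement timeline.
; The timeline's value, scaled by spline length, sets the cube's world position, while its rotation takes the spline's local roll and yaw with pitch held at zero.
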(event `self.trigger.OnComponentBeginOverlap`
  (params (OverlappedComponent :type "PrimitiveComponent Object Reference") (OtherActor :type "Actor Object Reference") (OtherComp :type "PrimitiveComponent Object Reference") (OtherBodyIndex :type Integer) (bFromSweep :type Boolean) (SweepResult :type "HitResult Structure (by ref)"))
  (bind _cube (`self.Cube`))
  (bind _spline (`self.Spline`))
  (cast `/Game/ThirdPerson/Blueprints/BP_ThirdPersonCharacter` OtherActor)
  (`/Engine/EditorBlueprintResources/StandardMacros.FlipFlop`
    (:`A`
      (bind (_direction _plateformway) (`Timeline|PlateformMovement` :!label _label)
        (:`Update`
          (bind _returnvalue (* _plateformway (`SplineComponent.GetSplineLength` _spline)))
          (`SceneComponent.K2_SetWorldLocation` _cube (`SplineComponent.GetLocationAtDistanceAlongSpline` _spline _returnvalue "World") false false)
          (bind (_returnvalue_roll _returnvalue_pitch _returnvalue_yaw) (`KismetMathLibrary.BreakRotator` (`SplineComponent.GetRotationAtDistanceAlongSpline` _spline _returnvalue "Local")))
          (`SceneComponent.K2_SetWorldRotation` _cube (`KismetMathLibrary.MakeRotator` _returnvalue_roll 0.0 _returnvalue_yaw) false false))))
    (:`B`
      (goto _label :!via `Reverse`))))

(fn `UserConstructionScript`)